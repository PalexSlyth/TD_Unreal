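; BP_Collectables is a pickup actor that flies to the player and is collected when the player pawn overlaps it.
; On overlap it stores its location, then a timeline alpha lerps it toward the pawn's current position each update.
; When the timeline finishes, it plays a 2D collect sound, calls ItemCompt on the player's BP_Pawn and destroys itself.
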(event Collision|EventActorBeginOverlap
  (params (OtherActor :type Actor%20Object%20Reference))
  ;[0 1 0.8743] Récupération et Destruction
  (if (== OtherActor (Game|Player|GetPlayerPawn 0))
    (Variables|Default|SetLerp%20Start%20Location (Transformation|GetActorLocation))
    (bind _smooth_lerp_alpha (Timeline|Alpha%20Blend%20Timeline Play)
      (:Update
        (Transformation|SetActorLocation (Math|Vector|Lerp(Vector) (Variables|Default|GetLerp%20Start%20Location) (Transformation|GetActorLocation (Game|Player|GetPlayerPawn 0)) _smooth_lerp_alpha) false false))
      (:Finished
        (Audio|PlaySound2D "/Game/Game/Sounds/Pickups/Stereo/Pickups_collect.Pickups_collect" 1.0 1.0 0.0 0 0)
        (bind _asbp_pawn (Utilities|Casting|CastToBP_Pawn (Game|GetPlayerCharacter 0)))
        (Default|ItemCompt _asbp_pawn)
        (Actor|DestroyActor)))))

(fn ConstructionScript)